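; BP_SwitchableBox is a light switch box that shows an on-screen prompt while an actor overlaps it.
; Overlap begin sets IsCanPressed and creates a WBP_PressedPerson widget, with Russian text "Включить свет" (turn on) when IsOn is true, otherwise "Выключить свет" (turn off).
; Overlap end clears the flag and removes the widget.
; Accessors expose IsCanPressed, IsOn and LightList; toggling the lights happens outside these graphs.
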(event `self.ReceiveActorBeginOverlap`
  (params (OtherActor :type "Actor Object Reference"))
  (set `self.IsCanPressed` true)
  (bind _returnvalue (`|CreateWidget` "/Game/SwitchLights/UI/WBP_PressedPerson.WBP_PressedPerson_C"))
  (`UserWidget.AddToViewport` _returnvalue 0)
  (if (`self.IsOn`)
    (bind _textlight (`/Game/SwitchLights/UI/WBP_PressedPerson.TextLight` _returnvalue))
    (`TextBlock.SetText` _textlight "Включить свет")
    (else
      (`TextBlock.SetText` _textlight "Выключить свет"))))

(event `self.ReceiveActorEndOverlap`
  (params (OtherActor :type "Actor Object Reference"))
  (set `self.IsCanPressed` false)
  (`Widget.RemoveFromParent` (stale `self.ReceiveActorBeginOverlap` _returnvalue)))

(fn `GetIsCanPrassed`
  (returns (IsCanPressed :type Boolean))
  (return (`self.IsCanPressed`)))

(fn `GetIsOn`
  (returns (NewParam :type Boolean))
  (return (`self.IsOn`)))

(fn `GetLightList`
  (returns (LightList :type "Array of /Game/SwitchLights/Blueprint/Object/Ligth/BP_Light Object Reference"))
  (return (`self.LightList`)))

(fn `SetIsOn`
  (params (IsOn :type Boolean))
  (set `self.IsOn` IsOn))

(fn `UserConstructionScript`)